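; awe_BP is a damageable actor, apparently an enemy, that is destroyed when its health runs out.
; AnyDamage subtracts incoming damage from a clamped Health value, guarded by an Isdead flag.
; At zero health it sets the flag, spawns Enemy_impact_BP at its own transform and destroys itself.
; BeginPlay, overlap, Tick and the construction script hold no logic.
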(event `self.ReceiveAnyDamage`
  (params (Damage :type "Float (single-precision)") (DamageType :type "DamageType Object Reference") (InstigatedBy :type "Controller Object Reference") (DamageCauser :type "Actor Object Reference"))
  ;[1 1 1] damage logic
  (if (not (`self.isdead?`))
    (bind _output_get (set `self.health` (`KismetMathLibrary.FClamp` (- (`self.health`) Damage) 0.0 5.0)))
    (if (== _output_get 0.0)
      (set `self.isdead?` true)
      (`|SpawnActorFromClass` "/Game/blueprints/enemy_impact_BP.enemy_impact_BP_C" (`self.GetTransform`) "Undefined" "OverrideRootScale" null null)
      (`self.K2_DestroyActor`))))

(fn `UserConstructionScript`)